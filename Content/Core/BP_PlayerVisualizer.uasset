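; BP_PlayerVisualizer is the visual side of a card-game player, handling the hand, draw animation and field slots.
; BeginPlay attaches a BP_HandGuide to the player's card-hand socket and spawns two centred rows of card slots, sized by Rules.MonsterZones.
; Draw montage notifies attach new cards to the hold socket, then refresh the hand guide and signal task completion.
; Turn is an empty stub, and SummonCard only handles monster-zone card materials.
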(event Custom|Draw
  (bind _notifyname (Animation|Montage|PlayMontage (Variables|/Script/Engine.Character|GetMesh (Variables|Default|GetPlayerRef)) "/Game/Characters/Mannequins/Animations/Quinn/human_duel_draw_hip_simple_Montage.human_duel_draw_hip_simple_Montage")
    (:OnNotifyBegin
      (switch name _notifyname
        (:TakeCard
          (for _array_element (Variables|/Script/HeroicNexus.BaseCharacter|GetHand (Variables|Default|GetPlayerRef))
            (if (not (Utilities|Array|ContainsItem (Variables|/Game/Core/BP_HandGuide.BP_HandGuide_C|GetCards (Variables|Default|GetVisualHand)) _array_element))
              (Transformation|AttachComponentToComponent _array_element (Variables|/Script/Engine.Character|GetMesh (Variables|Default|GetPlayerRef)) "card_hold" "SnapToTarget" "SnapToTarget" "SnapToTarget" true))))
        (:ReleaseCard
          (Variables|/Game/Core/BP_HandGuide.BP_HandGuide_C|SetCards (Variables|Default|GetVisualHand) (Variables|/Script/HeroicNexus.BaseCharacter|GetHand (Variables|Default|GetPlayerRef)))
          (Default|UpdateHand (Variables|Default|GetVisualHand))
          (Default|CallTaskComplete))))))

(event Custom|Turn
  (params (Phase :type EPhases%20Enum :default "PreDraw"))
  (switch Utilities|FlowControl|Switch|SwitchonEPhases Phase))

(event EventBeginPlay
  (bind _playerref (Variables|Default|GetPlayerRef))
  (bind _returnvalue (Game|SpawnActorfromClass "/Game/Core/BP_HandGuide.BP_HandGuide_C" (Math|Transform|MakeTransform "0, 0, 0" "0, 0, 0" "1.000000,1.000000,1.000000") "AlwaysSpawn" "MultiplyWithRoot" _playerref _playerref))
  (bind _output_get (Variables|Default|SetVisualHand _returnvalue))
  (Transformation|AttachComponentToComponent _output_get (Variables|/Script/Engine.Character|GetMesh (Variables|Default|GetPlayerRef)) "card_hand" "SnapToTarget" "SnapToTarget" "KeepRelative" true)
  (Variables|Default|SetisHumanPlayer (Pawn|IsLocallyControlled (Variables|Default|GetPlayerRef)))
  (CallFunction|CreatePlayerField false))

(fn ConstructionScript)

(fn CreatePlayerField
  (params (isTournament :type Boolean))
  (bind _rules (Variables|Default|GetRules))
  (bind _monsterzones (Utilities|Struct|BreakDuelRules _rules))
  (bind _returnvalue (- _monsterzones 1))
  (for _index (range 0 1)
    (for _index_2 (range 0 _returnvalue)
      (bind _returnvalue_2 (Game|SpawnActorfromClass "/Game/Core/BP_CardSlot.BP_CardSlot_C" (Math|Transform|MakeTransform (Transformation|GetWorldLocation (Variables|Default|GetArrow)) (Transformation|GetActorRotation) (Math|Conversions|ToVector(Float) (Math|Float|SelectFloat 0.4 0.25 isTournament))) "AlwaysSpawn" "MultiplyWithRoot" 0 0))
      (bind _output_get (LocalVariables|SetCardSlot _returnvalue_2))
      (Utilities|Array|Add (select (> _index 0) (Variables|Default|GetMonsterCards) (Variables|Default|GetChargeCards)) _output_get)
      (Transformation|AddActorWorldOffset (LocalVariables|GetCardSlot) (Math|Vector|MakeVector (.X (Class|KismetMathLibrary|BreakVector3f (+ (* (Transformation|GetActorForwardVector (LocalVariables|GetCardSlot)) (Math|Vector|MakeVector (* (* (.X (Class|KismetMathLibrary|BreakVector3f (.BoxExtent (Collision|GetActorBounds (LocalVariables|GetCardSlot) false false)))) 2.3) (+ _index 1)) (* (* (.X (Class|KismetMathLibrary|BreakVector3f (.BoxExtent (Collision|GetActorBounds (LocalVariables|GetCardSlot) false false)))) 2.3) (+ _index 1)) 1.0)) (* (Transformation|GetActorRightVector (LocalVariables|GetCardSlot)) (Math|Vector|MakeVector (* (* (.Y (Class|KismetMathLibrary|BreakVector3f (.BoxExtent (Collision|GetActorBounds (LocalVariables|GetCardSlot) false false)))) 2.3) (- _index_2 (/ _returnvalue 2))) (* (* (.Y (Class|KismetMathLibrary|BreakVector3f (.BoxExtent (Collision|GetActorBounds (LocalVariables|GetCardSlot) false false)))) 2.3) (- _index_2 (/ _returnvalue 2))) 1.0))))) (.Y (Class|KismetMathLibrary|BreakVector3f (+ (* (Transformation|GetActorForwardVector (LocalVariables|GetCardSlot)) (Math|Vector|MakeVector (* (* (.X (Class|KismetMathLibrary|BreakVector3f (.BoxExtent (Collision|GetActorBounds (LocalVariables|GetCardSlot) false false)))) 2.3) (+ _index 1)) (* (* (.X (Class|KismetMathLibrary|BreakVector3f (.BoxExtent (Collision|GetActorBounds (LocalVariables|GetCardSlot) false false)))) 2.3) (+ _index 1)) 1.0)) (* (Transformation|GetActorRightVector (LocalVariables|GetCardSlot)) (Math|Vector|MakeVector (* (* (.Y (Class|KismetMathLibrary|BreakVector3f (.BoxExtent (Collision|GetActorBounds (LocalVariables|GetCardSlot) false false)))) 2.3) (- _index_2 (/ _returnvalue 2))) (* (* (.Y (Class|KismetMathLibrary|BreakVector3f (.BoxExtent (Collision|GetActorBounds (LocalVariables|GetCardSlot) false false)))) 2.3) (- _index_2 (/ _returnvalue 2))) 1.0))))) 0.0)))))

(fn SummonCard
  (params (Card :type Card%20Object%20Reference))
  (switch Utilities|FlowControl|Switch|SwitchonELocations (.Location (Utilities|Struct|BreakCardState (Variables|/Script/HeroicNexus.Card|GetCurrentState Card)))
    (:MZone
      (bind _array_element (Utilities|Array|ForEachLoopwithBreak (Variables|Default|GetMonsterCards) :!label _label)
        (:LoopBody
          (Utilities|IsValid _array_element
            (:Is%20Not%20Valid
              (Default|SetCardMaterial _array_element "/Game/Core/CardFront.CardFront")
              (goto _label Break))))))))