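; BP_HandGuide is an actor that lays out a hand of cards along an arched spline.
; UpdateHand stretches the spline with the card count and raises its midpoint through a clamped range mapping, so larger hands arch more.
; It attaches each card to the spline, spaced evenly by distance with curve-following rotation and hand scale, with a single card handled separately.
; The event graph is empty and the construction script's UpdateHand call is disconnected.
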(event EventBeginPlay)

(event Collision|EventActorBeginOverlap
  (params (OtherActor :type Actor%20Object%20Reference)))

(event EventTick
  (params (DeltaSeconds :type Float%20%28single-precision%29)))

(fn ConstructionScript)

(fn UpdateHand
  (Variables|Default|SetNumCards (Utilities|Array|Length (Variables|Default|GetCards)))
  ;[0 0 0] Update spline points
  (Spline|SetLocationatSplinePoint (Variables|Default|GetSpline) 2 (* (Math|Vector|MakeVector 2.0 0.0 0.0) (Variables|Default|GetNumCards)) "Local" true)
  (Spline|SetLocationatSplinePoint (Variables|Default|GetSpline) 1 (+ (/ (Spline|GetLocationatSplinePoint (Variables|Default|GetSpline) 2 "Local") (Math|Float|MakeLiteralFloat 2.0)) (Math|Vector|MakeVector 0.0 0.0 (Math|Float|MapRangeClamped (Math|Conversions|ToFloat(Integer) (Variables|Default|GetNumCards)) 1.0 1e+01 0.0 1.0))) "Local" true)
  ;[0 0 0] Spawn cards
  (if (> (Variables|Default|GetNumCards) 0)
    (if (> (Variables|Default|GetNumCards) 1)
      (LocalVariables|SetDist (/ (Spline|GetSplineLength (Variables|Default|GetSpline)) (- (Variables|Default|GetNumCards) 1)))
      (for _index (range 0 (- (Utilities|Array|Length (Variables|Default|GetCards)) 1))
        (bind _output_get (LocalVariables|SetIndex _index))
        (LocalVariables|SetCard (Utilities|Array|Get(acopy) (Variables|Default|GetCards) _output_get))
        (Transformation|AttachComponentToComponent (LocalVariables|GetCard) (Variables|Default|GetSpline) "None" "SnapToTarget" "SnapToTarget" "SnapToTarget" true)
        (Transformation|SetActorRelativeTransform (LocalVariables|GetCard) (Math|Transform|MakeTransform (.Location (Math|Transform|BreakTransform (Spline|GetTransformatDistanceAlongSpline (Variables|Default|GetSpline) (* (LocalVariables|GetIndex) (LocalVariables|GetDist)) "Local" false))) (.Rotation (Math|Transform|BreakTransform (Spline|GetTransformatDistanceAlongSpline (Variables|Default|GetSpline) (* (LocalVariables|GetIndex) (LocalVariables|GetDist)) "Local" false))) (Math|Conversions|ToVector(Float) (Class|BPFHeroicNexus|GetCardHandScale))) false false)
        (Transformation|AddActorLocalRotation (LocalVariables|GetCard) "90.000000,-90.000000,1.000000" false false))
      (else
        (LocalVariables|SetCard (Utilities|Array|Get(acopy) (Variables|Default|GetCards)))
        (Transformation|AttachComponentToComponent (LocalVariables|GetCard) (Variables|Default|GetSpline) "None" "SnapToTarget" "SnapToTarget" "SnapToTarget" true)
        (Transformation|SetActorRelativeTransform (LocalVariables|GetCard) (Math|Transform|MakeTransform "0, 0, 0" "0.000000,-90.000000,0.000000" (Math|Conversions|ToVector(Float) (Class|BPFHeroicNexus|GetCardHandScale))) false false)))))