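; BP_Duel is a duel Blueprint that starts a duel as soon as it begins play.
; BeginPlay runs the parent logic, calls an empty MovePlayersIntoPosition event, then calls StartDuel, which is not defined in this graph.
; A disconnected chain would AI-move every player to one hardcoded point and start the duel once all arrive, but it never runs.
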(event Custom|MovePlayersIntoPosition)

(event EventBeginPlay
  (|CallParentFunction)
  (CallFunction|MovePlayersIntoPosition)
  (Class|Duel|StartDuel))

(fn ConstructionScript)