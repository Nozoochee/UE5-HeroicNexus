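; Base card Blueprint that represents one card by ID, with stats, artwork, effects and an optional monster mesh.
; LoadData queries Cards.db by ID to seed original, current and previous state, then pulls soft art and mesh references from DT_CardArt.
; BeginPlay runs that load, instantiates effect objects from BaseEffects and async-loads art into a dynamic material's Front texture.
; LoadArtAndMeshes async-loads the art again, plus any monster mesh, which it unhides.
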(event Custom|LoadArtAndMeshes
  (bind _monstermesh (Variables|Default|GetMonsterMesh))
  ;[0 0 0] Asnyc loading
  (bind _object (Utilities|AsyncLoadAsset (Variables|Default|GetCardArt))
    (:then
      (if (Utilities|IsValidSoftObjectReference _monstermesh)
        (bind _object_2 (Utilities|AsyncLoadAsset _monstermesh)
          (:Completed
            (Components|SkeletalMesh|SetSkeletalMeshAsset (Variables|Default|GetSkeletalMesh) (.AsSkeletal%20Mesh (Utilities|Casting|CastToSkeletalMesh _object_2)))
            (Development|SetHiddeninGame (Variables|Default|GetSkeletalMesh) false false)))))
    (:Completed
      (Rendering|Material|SetTextureParameterValue (Variables|Default|GetDynamicMaterial) "Front" (.AsTexture (Utilities|Casting|CastToTexture _object))))))

(event EventBeginPlay
  (bind _returnvalue (Rendering|Material|CreateDynamicMaterialInstance (Variables|Default|GetCardMesh) 0 0 "None" :!class /Script/Engine.PrimitiveComponent))
  (Variables|Default|SetDynamicMaterial _returnvalue)
  (CallFunction|LoadData)
  (for _array_element (Variables|Default|GetBaseEffects)
    (bind _returnvalue_2 (Game|ConstructObjectfromClass _array_element self (Variables|Default|GetField)))
    (Utilities|Array|Add (Variables|Default|GetAvailableEffects) _returnvalue_2))
  (bind _object (Utilities|AsyncLoadAsset (Variables|Default|GetCardArt))
    (:Completed
      (Rendering|Material|SetTextureParameterValue (Variables|Default|GetDynamicMaterial) "Front" (.AsTexture (Utilities|Casting|CastToTexture _object))))))

(fn ConstructionScript)

(fn LoadData
  (bind _returnvalue (Class|DbManagerStatics|GetDatabasebyFilename "Cards.db"))
  (Utilities|IsValid _returnvalue
    (:Is%20Valid
      (bind _asdata_access_layer_bp (Utilities|Casting|CastToDataAccessLayerBP _returnvalue))
      (bind _output_get (LocalVariables|SetStatement (Class|PreparedStatementManager|FindStatement (Variables|/Script/SqliteGameDB.DbBase|GetQueryManager _asdata_access_layer_bp) "GetCardByID")))
      (Class|DbStatement|SetIntParameterValue _output_get "@ID" (Variables|Default|GetID))
      (bind _returnvalue_2 (Class|DbStatement|ExecuteSelect (LocalVariables|GetStatement)))
      (if (> (Utilities|Array|Length (Utilities|Struct|BreakQueryResult _returnvalue_2)) 0)
        (bind _output_get_2 (Variables|Default|SetOriginalData (Utilities|Struct|MakeCardData (Variables|Default|GetID) (Math|Conversions|ToInteger(Byte) (.IntVal (Utilities|Struct|BreakQueryResultField (Utilities|Array|Get(acopy) (Utilities|Struct|BreakQueryResultRow (Utilities|Array|Get(acopy) (Utilities|Struct|BreakQueryResult _returnvalue_2))) 4)))) (Math|Conversions|ToInteger(Byte) (.IntVal (Utilities|Struct|BreakQueryResultField (Utilities|Array|Get(acopy) (Utilities|Struct|BreakQueryResultRow (Utilities|Array|Get(acopy) (Utilities|Struct|BreakQueryResult _returnvalue_2))) 5)))) (Math|Conversions|ToInteger(Byte) (.IntVal (Utilities|Struct|BreakQueryResultField (Utilities|Array|Get(acopy) (Utilities|Struct|BreakQueryResultRow (Utilities|Array|Get(acopy) (Utilities|Struct|BreakQueryResult _returnvalue_2))) 6)))) (Math|Conversions|ToInteger(Byte) (.IntVal (Utilities|Struct|BreakQueryResultField (Utilities|Array|Get(acopy) (Utilities|Struct|BreakQueryResultRow (Utilities|Array|Get(acopy) (Utilities|Struct|BreakQueryResult _returnvalue_2))) 7)))) (Math|Conversions|ToInteger(Byte) (.IntVal (Utilities|Struct|BreakQueryResultField (Utilities|Array|Get(acopy) (Utilities|Struct|BreakQueryResultRow (Utilities|Array|Get(acopy) (Utilities|Struct|BreakQueryResult _returnvalue_2))) 8)))) (Utilities|Text|ToText(String) (.StrVal (Utilities|Struct|BreakQueryResultField (Utilities|Array|Get(acopy) (Utilities|Struct|BreakQueryResultRow (Utilities|Array|Get(acopy) (Utilities|Struct|BreakQueryResult _returnvalue_2))) 1)))) (Utilities|Text|ToText(String) (.StrVal (Utilities|Struct|BreakQueryResultField (Utilities|Array|Get(acopy) (Utilities|Struct|BreakQueryResultRow (Utilities|Array|Get(acopy) (Utilities|Struct|BreakQueryResult _returnvalue_2))) 2)))))))
        (bind _output_get_3 (Variables|Default|SetCurrentState (Utilities|Struct|MakeCardState (.Id (Utilities|Struct|BreakCardData _output_get_2)) (.Type (Utilities|Struct|BreakCardData _output_get_2)) (.Atk (Utilities|Struct|BreakCardData _output_get_2)) (.Atk (Utilities|Struct|BreakCardData _output_get_2)) (.Def (Utilities|Struct|BreakCardData _output_get_2)) (.Def (Utilities|Struct|BreakCardData _output_get_2)) (.Cost (Utilities|Struct|BreakCardData _output_get_2)) (.Cost (Utilities|Struct|BreakCardData _output_get_2)))))
        (Variables|Default|SetPreviousState _output_get_3)
        (bind _returnvalue_3 (Utilities|GetDataTableRow "/Game/Core/Cards/DT_CardArt.DT_CardArt" (Utilities|String|StringToName (Utilities|String|ToString(Integer) (Variables|Default|GetID))))
          (:then
            (Variables|Default|SetCardArt (.CardArt (Utilities|Struct|BreakCardArtTable _returnvalue_3)))
            (Variables|Default|SetMonsterMesh (.Mesh (Utilities|Struct|BreakCardArtTable _returnvalue_3)))))
        (else
          (Development|PrintString "Card not found in DB"))))
    (:Is%20Not%20Valid
      (Development|PrintString "NO CARD DB"))))