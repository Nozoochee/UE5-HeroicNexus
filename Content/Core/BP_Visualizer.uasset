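; BP_Visualizer plays back queued card-duel operations as on-screen announcements and player animations.
; RunAllVisualizations pops VisualizeOperations recursively: turns announce the phase (continuing only for Draw), draws await the player's BP_PlayerVisualizer TaskComplete, and an empty queue calls FinishedCatchingUp.
; Duel start and global announcements share the main UI's DuelStartAnim.
; Summon handling is unwired, and BeginPlay draws a debug facing arrow.
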(event Custom|TaskComplete_Event
  (EventDispatchers|UnbindEventfromTaskComplete (Variables|Default|GetPlayerVisualizer) (delegate Custom|TaskComplete_Event))
  (CallFunction|RunAllVisualizations))

(event Custom|RunAllVisualizations
  (if (> (Utilities|Array|Length (Variables|Default|GetVisualizeOperations)) 0)
    (bind _output_get (Variables|Default|SetCurrentVisualization (Utilities|Array|Get(acopy) (Variables|Default|GetVisualizeOperations))))
    (Utilities|Array|RemoveIndex (Variables|Default|GetVisualizeOperations))
    (switch Utilities|FlowControl|Switch|SwitchonEProcess (.Type (Utilities|Struct|BreakProcessUnit (.Process (Utilities|Struct|BreakDuelOperation _output_get))))
      (:Turn
        (CallFunction|ShowAnnouncementGlobal (Utilities|Text|ToText(String) (Utilities|String|EnumtoString (.Phase (Utilities|Struct|BreakDuelInfo (Class|PlayField|GetTurnInfo (Variables|Default|GetField)))))))
        (switch Utilities|FlowControl|Switch|SwitchonEPhases (.Phase (Utilities|Struct|BreakDuelInfo (Class|PlayField|GetTurnInfo (Variables|Default|GetField))))
          (:Draw
            (CallFunction|RunAllVisualizations))))
      (:Draw
        (CallFunction|SetPlayerVisualizer (Utilities|Array|Get(acopy) (.Targets (Utilities|Struct|BreakProcessUnit (.Process (Utilities|Struct|BreakDuelOperation _output_get))))))
        (EventDispatchers|AssignTaskComplete (Variables|Default|GetPlayerVisualizer) (delegate Custom|TaskComplete_Event))
        (Default|Draw (Variables|Default|GetPlayerVisualizer))))
    (else
      (Class|FieldVisualizer|FinishedCatchingUp))))

(event Custom|ShowAnnouncementGlobal
  (params (Annoucement :type Text))
  ;[0 0 0] For showing info to both players regardless of whose turn it is (e.g. new turn phase)
  (bind _asbp_player_controller (Utilities|Casting|CastToBP_PlayerController (Game|GetPlayerController 0)))
  (Rendering|Components|TextRender|SetText (Variables|/Game/Core/UI/BPI_MainUI.BPI_MainUI_C|GetDuelText (Variables|/Game/Core/Characters/Player/BP_PlayerController.BP_PlayerController_C|GetMainUI _asbp_player_controller)) Annoucement)
  (Components|Animation|PlayAnimation (Variables|/Game/Core/Characters/Player/BP_PlayerController.BP_PlayerController_C|GetMainUI _asbp_player_controller) (Variables|/Game/Core/UI/BPI_MainUI.BPI_MainUI_C|GetDuelStartAnim (Variables|/Game/Core/Characters/Player/BP_PlayerController.BP_PlayerController_C|GetMainUI _asbp_player_controller)) 0.0))

(event EventBeginPlay
  (bind _returnvalue (Transformation|GetActorLocation))
  (Rendering|Debug|DrawDebugArrow _returnvalue (+ _returnvalue (* (Transformation|GetActorForwardVector) 2e+02)) 5e+02 "(R=0.484375,G=0.000000,B=0.032218,A=1.000000)" 3.0 2.0))

(event EventStartVisualization
  (CallFunction|RunAllVisualizations))

(event EventStartHumanPlayerDuelUI
  (bind _returnvalue (Game|GetPlayerController 0))
  (bind _asbp_player_controller (Utilities|Casting|CastToBP_PlayerController _returnvalue))
  (bind _mainui (Variables|/Game/Core/Characters/Player/BP_PlayerController.BP_PlayerController_C|GetMainUI _asbp_player_controller))
  (Components|Animation|PlayAnimation _mainui (Variables|/Game/Core/UI/BPI_MainUI.BPI_MainUI_C|GetDuelStartAnim _mainui) 0.0
    (:Finished
      (|CallParentFunction))))

(fn ConstructionScript)

(fn SetPlayerVisualizer
  (params (Player :type Object%20Object%20Reference))
  (bind _asbase_character (Utilities|Casting|CastToBaseCharacter Player))
  (Variables|Default|SetPlayerVisualizer (.AsBP%20Player%20Visualizer (Utilities|Casting|CastToBP_PlayerVisualizer (.Value (Utilities|Map|Find (Variables|Default|GetPlayerVisualizers) _asbase_character))))))